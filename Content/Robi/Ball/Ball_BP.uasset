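; Ball Blueprint, apparently meant as a physics ball that is pushed at start and keeps its momentum through bounces.
; All events and the construction script are empty, so none of the movement logic currently runs.
; Disconnected nodes hold an initial velocity-change impulse and two routines that randomly adjust BallSpeed, then clamp the physics velocity to that magnitude.
; One of those routines prints a top-wall debug message.
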(event Custom|TopScreenTrigger)

(event EventBeginPlay
  ;[1 1 1] Pushes ball at start
)

(event Collision|EventActorBeginOverlap
  (params (OtherActor :type Actor%20Object%20Reference)))

(event Collision|EventHit
  (params (MyComp :type Primitive%20Component%20Object%20Reference) (Other :type Actor%20Object%20Reference) (OtherComp :type Primitive%20Component%20Object%20Reference) (bSelfMoved :type Boolean) (HitLocation :type Vector :default "0, 0, 0") (HitNormal :type Vector :default "0, 0, 0") (NormalImpulse :type Vector :default "0, 0, 0") (Hit :type Hit%20Result%20Structure%20%28by%20ref%29))
  ;[1 1 1] Keeps ball momentume
)

(fn ConstructionScript)